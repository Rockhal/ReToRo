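; Pose-matching wall obstacle that repeatedly slides toward negative X and damages the player whose dance does not match it.
; After a five-second delay, Tick moves the mesh; past an X limit it teleports back, speeds up and rerolls its type.
; WallType reveals one of four pose meshes, with both 3 and 4 showing Cha.
; The Box overlap compares the player's Dance to WallType exactly, calling Damage on a mismatch.
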(event `self.ReceiveBeginPlay`
  (bind _asbp_player (cast `/Game/ThirdPerson/Blueprints/BP_Player` (`GameplayStatics.GetPlayerPawn` 0)))
  (set `self.As BP Player` _asbp_player)
  (set `self.Fst_pos` (`SceneComponent.GetSocketLocation` (`self.StaticMesh`) "None"))
  (set `self.WallType` (`KismetMathLibrary.RandomInteger` 5))
  (`KismetSystemLibrary.Delay` 5.0)
  (`self.SetActorTickEnabled` true)
  (`SceneComponent.SetHiddenInGame` (`self.posewall_back`) true false :!label _label)
  (`SceneComponent.SetHiddenInGame` (`self.posewall_cha`) true false)
  (`SceneComponent.SetHiddenInGame` (`self.posewall_Jump`) true false)
  (`SceneComponent.SetHiddenInGame` (`self.posewall_ku`) true false)
  (switch `int` (`self.WallType`)
    (:`Default`
      (`SceneComponent.SetHiddenInGame` (`self.posewall_cha`) false false))
    (:`0`
      (`SceneComponent.SetHiddenInGame` (`self.posewall_Jump`) false false))
    (:`1`
      (`SceneComponent.SetHiddenInGame` (`self.posewall_ku`) false false))
    (:`2`
      (`SceneComponent.SetHiddenInGame` (`self.posewall_back`) false false))))

(event `self.ReceiveTick`
  (params (DeltaSeconds :type "Float (single-precision)"))
  (bind _returnvalue_x (`KismetMathLibrary.BreakVector` (`SceneComponent.GetSocketLocation` (`self.StaticMesh`) "None")))
  (`SceneComponent.K2_AddRelativeLocation` (`self.StaticMesh`) (`KismetMathLibrary.MakeVector` (`self.WallSpeed`)) true false)
  (if (< _returnvalue_x -3900.0)
    (`KismetSystemLibrary.PrintString` "壁の位置をリセットする" true true (struct :`G` 0.66 :`B` 1.0 :`A` 1.0) 0.2)
    (`SceneComponent.K2_SetWorldLocation` (`self.StaticMesh`) (`self.Fst_pos`) false true)
    (set `self.WallSpeed` (+ (`self.WallSpeed`) -2.0))
    (set `self.WallType` (`KismetMathLibrary.RandomInteger` 5))
    (goto _label)))

(event `self.StaticMesh.OnComponentHit`
  (params (HitComponent :type "PrimitiveComponent Object Reference") (OtherActor :type "Actor Object Reference") (OtherComp :type "PrimitiveComponent Object Reference") (NormalImpulse :type "Vector Structure") (Hit :type "HitResult Structure (by ref)")))

(event `self.posewall_Jump.OnComponentBeginOverlap`
  (params (OverlappedComponent :type "PrimitiveComponent Object Reference") (OtherActor :type "Actor Object Reference") (OtherComp :type "PrimitiveComponent Object Reference") (OtherBodyIndex :type Integer) (bFromSweep :type Boolean) (SweepResult :type "HitResult Structure (by ref)")))

(event `self.Box.OnComponentBeginOverlap`
  (params (OverlappedComponent :type "PrimitiveComponent Object Reference") (OtherActor :type "Actor Object Reference") (OtherComp :type "PrimitiveComponent Object Reference") (OtherBodyIndex :type Integer) (bFromSweep :type Boolean) (SweepResult :type "HitResult Structure (by ref)"))
  (bind _as_bp_player (`self.As BP Player`))
  (bind _as_bp_player_2 (`self.As BP Player`))
  (if (`self.ActorHasTag` OtherActor "player")
    (`/Engine/EditorBlueprintResources/StandardMacros.IsValid` _as_bp_player ; プレイヤーのアニメなにしてる
      (:`Is Valid`
        (if (== (`/Game/ThirdPerson/Blueprints/BP_Player.Dance` _as_bp_player) (`self.WallType`))
          (`KismetSystemLibrary.PrintString` "壁を潜り抜けた" true true (struct :`G` 0.66 :`B` 1.0 :`A` 1.0) 0.8 "kabe")
          (else
            (`KismetSystemLibrary.PrintString` "壁に触れた" true true (struct :`G` 0.66 :`B` 1.0 :`A` 1.0) 0.8 "kabe")
            (`|ExecutionSequence`
              (:`then_0`
                (`/Engine/EditorBlueprintResources/StandardMacros.IsValid` _as_bp_player_2 ; プレイヤーにダメージ送る
                  (:`Is Valid`
                    (`/Game/ThirdPerson/Blueprints/BP_Player.Damage` _as_bp_player_2)))))))))))

(fn `UserConstructionScript`)