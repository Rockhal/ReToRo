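; BP_GameMode is a game mode that runs a countdown timer and tracks the player's life count.
; Tick subtracts delta time from GameTimer and prints it, then uses a DoOnce to print a game over message and set IsGamOver once the timer drops below zero.
; A DecreaseLife event decrements Life, which does not affect the game over flag here.
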(event `self.ReceiveTick`
  (params (DeltaSeconds :type "Float (single-precision)"))
  (if (< (`self.GameTimer`) 0.0)
    ; ゲームオーバーのフラグをセット
    (`/Engine/EditorBlueprintResources/StandardMacros.DoOnce` false
      (:`Completed`
        (`KismetSystemLibrary.PrintString` "ゲームオーバー")
        (set `self.IsGamOver` true)))
    (else
      ; ゲームカウントダウン
      (bind _output_get (set `self.GameTimer` (- (`self.GameTimer`) DeltaSeconds)))
      (`KismetSystemLibrary.PrintString` (`KismetStringLibrary.Conv_DoubleToString` _output_get)))))

(event `DecreaseLife`
  (bind _result (`/Engine/EditorBlueprintResources/StandardMacros.DecrementFloat` (`self.Life`))
    (:`  `
      (set `self.Life` _result))))

(fn `UserConstructionScript`)