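; Game mode that holds the player's Life and Stamina, game-over and clear state, and the HUD and result widgets.
; BeginPlay caches starting values as maximums, and decrease events update the HUD bars as ratios of them.
; Tick sets the game-over flag once when Life runs out, and any key opens L_Title after game over or clear.
; Separate Show events create the in-game, clear and game-over widgets, the latter two hiding the HUD.
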(event `self.ReceiveTick`
  (params (DeltaSeconds :type "Float (single-precision)"))
  ; ゲームオーバー判定
  (if (<= (`self.Life`) 0.0)
    ; ゲームオーバーのフラグをセット
    (`/Engine/EditorBlueprintResources/StandardMacros.DoOnce` false
      (:`Completed`
        (`KismetSystemLibrary.PrintString` "ゲームオーバー")
        (set `self.IsGamOver` true)))))

(event `Key|AnyKey`
  (params (Key :type "Key Structure"))
  ; ゲームクリア、オーバー時に何かしらのキーを押すことで、タイトルレベルに遷移
  (:`Pressed`
    (if (or (`self.IsGamOver`) (`self.IsGameClear`))
      (`GameplayStatics.OpenLevelBySoftObjectPtr` "/Game/Levels/L_Title.L_Title"))))

(event `self.ReceiveBeginPlay`
  ; 初期化処理
  (set `self.MaxLife` (`self.Life`)) ; 最大のライフ値を保存
  (set `self.MaxStamina` (`self.Stamina`)) ; 最大のスタミナ値を保存
)

(event `ShowGameClear`
  ; ゲームクリアUI表示
  (`Widget.SetVisibility` (`self.InGameView`) "Hidden") ; インゲームを非表示に
  (bind _returnvalue (`|CreateWidget` "/Game/UI/WBP_GameClear.WBP_GameClear_C"))
  (bind _output_get (set `self.GameClearView` _returnvalue))
  (`UserWidget.AddToViewport` _output_get 0))

(event `ShowInGameView`
  ; インゲームUI作成
  (bind _returnvalue (`|CreateWidget` "/Game/UI/WBP_InGame.WBP_InGame_C"))
  (bind _output_get (set `self.InGameView` _returnvalue))
  (`UserWidget.AddToViewport` _output_get 0))

(event `ShowGameOver`
  ; ゲームオーバーUI表示
  (`Widget.SetVisibility` (`self.InGameView`) "Hidden") ; インゲームを非表示に
  (bind _returnvalue (`|CreateWidget` "/Game/UI/WBP_GameOver.WBP_GameOver_C"))
  (bind _output_get (set `self.GameOverView` _returnvalue))
  (`UserWidget.AddToViewport` _output_get 0))

(event `DecreaseLife`
  ; ライフの減少
  (bind _result (`/Engine/EditorBlueprintResources/StandardMacros.DecrementFloat` (`self.Life`))
    (:`  `
      (set `self.Life` _result)
      ; ライフバーの減少処理
      (`ProgressBar.SetPercent` (`/Game/UI/WBP_InGame.LifeBar` (`self.InGameView`)) (`KismetMathLibrary.SafeDivide` (`self.Life`) (`self.MaxLife`))))))

(event `DecreaseStamina`
  (params (DecreaseVal :type "Float (double-precision)"))
  ; スタミナの減少
  (set `self.Stamina` (- (`self.Stamina`) DecreaseVal))
  ; スタミナバーの減少表示
  (`ProgressBar.SetPercent` (`/Game/UI/WBP_InGame.StaminerBar` (`self.InGameView`)) (`KismetMathLibrary.SafeDivide` (`self.Stamina`) (`self.MaxStamina`))))

(fn `UserConstructionScript`)